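; BP_Tile is a tile actor with a Highlight component that shows whether the tile is selected.
; The construction script creates a dynamic material instance from the highlight's first material, stores it and applies it to the highlight.
; ToggleSelected flips IsSelected and shows or hides the highlight in game through two helper functions.
; BeginPlay, overlap and Tick events are unused.
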(event EventBeginPlay)

(event Collision|EventActorBeginOverlap
  (params (OtherActor :type Actor%20Object%20Reference)))

(event EventTick
  (params (DeltaSeconds :type Float%20%28single-precision%29)))

(event EventToggleSelected
  (if (Variables|Default|GetbIsSelected self)
    (CallFunction|SetHighlightNotVisible)
    (else
      (CallFunction|SetHighlightVisible)))
  (Variables|Default|SetbIsSelected (not (Variables|Default|GetbIsSelected self))))

(fn ConstructionScript
  (bind _returnvalue (Rendering|Material|CreateDynamicMaterialInstance (Utilities|Array|Get(acopy) (Rendering|Material|GetMaterials (Variables|Default|GetHighlight))) "None" :!class /Script/Engine.KismetMaterialLibrary))
  (bind _output_get (Variables|Default|SetMaterial _returnvalue))
  (Rendering|Material|SetMaterial (Variables|Default|GetHighlight) 0 _output_get))

(fn SetHighlightVisible
  (Development|SetHiddeninGame (Variables|Default|GetHighlight) false false))

(fn SetHighlightNotVisible
  (Development|SetHiddeninGame (Variables|Default|GetHighlight) true false))