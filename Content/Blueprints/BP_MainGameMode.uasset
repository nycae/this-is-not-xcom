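; Game mode for a turn-based army game that rotates turns among TeamLeader teams, starting with the player.
; BeginPlay creates the score manager and player GUI, then binds turn and unit-death delegates on every team.
; Turn starts refill unit energy and hand non-player armies to the AI assistant; turn ends pass play round-robin.
; Deaths free tiles and eliminate empty teams, ending the game at one team or the turn limit.
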(event Custom|AttendEndOfTurn
  (params (Team :type Team%20Leader%20Object%20Reference))
  (bind _teams (Variables|Default|GetTeams))
  (bind _returnvalue (Utilities|Array|Length _teams))
  (if (<= _returnvalue 1)
    (Default|CallOnEndGame (Utilities|Array|Get(acopy) _teams))
    (else
      (Math|Integer|IncrementInt (Variables|Default|GetTurnCounter)
        (:%20%20
          (bind _output_get (Variables|Default|SetTurnHolder (Utilities|Array|Get(acopy) _teams (Math|Integer|%(Integer) (+ (Utilities|Array|FindItem _teams Team) 1) _returnvalue))))
          (Class|TeamLeader|GrantTurn _output_get))))))

(event Custom|AttendTurnBegin
  (params (Team :type Team%20Leader%20Object%20Reference))
  (bind _army (Variables|/Script/ThisisNotXcom.TeamLeader|GetArmy Team))
  (Utilities|FlowControl|Sequence
    (:then_0
      (if (>= (Variables|Default|GetTurnCounter) (Variables|Default|GetMaxTurns))
        (Default|CallOnEndGame)))
    (:then_1
      (Variables|Default|SetLastTurnTimestamp (Utilities|Time|GetWorldDeltaSeconds)))
    (:then_2
      (for _array_element _army
        (Variables|/Script/ThisisNotXcom.Unit|SetEnergy _array_element (Variables|/Script/ThisisNotXcom.Unit|GetMaxEnergy _array_element))))
    (:then_3
      (if (not (Actor|ActorHasTag Team "Player"))
        (Class|AIPlayer|TimerforDelayedExecution (Variables|Default|GetAIAssistant) _army)))))

(event Custom|AttendDeath
  (params (Unit :type Unit%20Object%20Reference) (Team :type Team%20Leader%20Object%20Reference))
  (bind _location (Variables|/Script/ThisisNotXcom.Unit|GetLocation Unit))
  (bind _teams (Variables|Default|GetTeams))
  (Utilities|FlowControl|Sequence
    (:then_0
      (Utilities|Array|RemoveItem (Variables|/Script/ThisisNotXcom.TeamLeader|GetArmy Team) Unit)
      (Variables|/Script/ThisisNotXcom.Tile|SetOcupant _location 0)
      (Variables|/Script/ThisisNotXcom.Tile|SetState _location "TS_Empty"))
    (:then_1
      (Rendering|SetActorHiddenInGame Unit true)
      (Actor|DestroyActor Unit))
    (:then_2
      (if (== (Utilities|Array|Length (Variables|/Script/ThisisNotXcom.TeamLeader|GetArmy Team)) 0)
        (Utilities|Array|RemoveItem _teams Team)
        (if (== (Utilities|Array|Length _teams) 1)
          (Default|CallOnEndGame (Utilities|Array|Get(acopy) _teams)))))))

(event EventBeginPlay
  (CallFunction|FindAIandConstructScoreManager)
  (CallFunction|AddUserInterfacetoPlayer)
  (CallFunction|FindTeamsandInstallHandlers (delegate Custom|AttendTurnBegin) (delegate Custom|AttendEndOfTurn) (delegate Custom|AttendDeath))
  (Class|TeamLeader|GrantTurn (Variables|Default|GetTurnHolder)))

(event EventTick
  (params (DeltaSeconds :type Float%20%28single-precision%29))
  (if (> DeltaSeconds (+ (Variables|Default|GetMaxTurnTime) (Variables|Default|GetLastTurnTimestamp)))
    (Class|TeamLeader|FinishTurn (Variables|Default|GetTurnHolder))))

(fn ConstructionScript)

(fn SelectNewTurnHolder
  (params (CurrentHolder :type Team%20Leader%20Object%20Reference))
  (bind _teams (Variables|Default|GetTeams))
  (bind _output_get (Variables|Default|SetTurnHolder (Utilities|Array|Get(acopy) _teams (Math|Integer|%(Integer) (+ (Utilities|Array|FindItem _teams CurrentHolder) 1) (Utilities|Array|Length _teams)))))
  (Class|TeamLeader|GrantTurn _output_get))

(fn StoreResults
  (for _array_element (Variables|Default|GetTeams)
    (Class|ScoreManager|UpdateScore (Variables|Default|GetScoreManager) (Variables|/Script/ThisisNotXcom.TeamLeader|GetPlayerName _array_element) (+ (Variables|/Script/ThisisNotXcom.TeamLeader|GetScore _array_element) (Class|TeamLeader|HealthOfUnits _array_element)))))

(fn FindAIandConstructScoreManager
  (bind _outactors (Actor|GetAllActorsOfClass "/Script/ThisisNotXcom.AIPlayer"))
  (Variables|Default|SetAIAssistant (Utilities|Array|Get(acopy) _outactors))
  (bind _returnvalue (Game|ConstructObjectfromClass "/Script/ThisisNotXcom.ScoreManager" self))
  (Variables|Default|SetScoreManager _returnvalue))

(fn AddUserInterfacetoPlayer
  (bind _outactors (Actor|GetAllActorswithTag "Player"))
  (bind _asteam_leader (Utilities|Casting|CastToTeamLeader (Utilities|Array|Get(acopy) _outactors))
    (:then
      (bind _output_get (Variables|Default|SetTurnHolder _asteam_leader))
      (bind _returnvalue (Game|ConstructObjectfromClass "/Game/Blueprints/UserInterface/Gameplay/BP_PlayerGUI.BP_PlayerGUI_C" (Pawn|GetController _output_get)))
      (Default|AddTeam _returnvalue _output_get)
      (UserInterface|Viewport|AddtoViewport _returnvalue 0))
    (:CastFailed
      _))
  (return))

(fn FindTeamsandInstallHandlers
  (params (Begin%20Turn%20Delegate :type Delegate%20%28by%20ref%29) (Turn%20End%20Delegate :type Delegate%20%28by%20ref%29) (Unit%20Death%20Delegate :type Delegate%20%28by%20ref%29))
  (bind _outactors (Actor|GetAllActorsOfClass "/Script/ThisisNotXcom.TeamLeader"))
  (for _array_element _outactors
    (Utilities|FlowControl|Sequence
      (:then_0
        (Utilities|Array|Add (Variables|Default|GetTeams) _array_element)
        (EventDispatchers|BindEventtoBeginTurn _array_element Begin%20Turn%20Delegate)
        (EventDispatchers|BindEventtoTurnEnd _array_element Turn%20End%20Delegate))
      (:then_1
        (for _array_element_2 (Variables|/Script/ThisisNotXcom.TeamLeader|GetArmy _array_element)
          (EventDispatchers|BindEventtoOnDeath _array_element_2 Unit%20Death%20Delegate))))))