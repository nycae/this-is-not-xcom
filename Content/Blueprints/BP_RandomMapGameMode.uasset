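; BP_RandomMapGameMode is the game mode for random-map, turn-based team play, opening with a player unit deployment screen.
; On BeginPlay it sets up the AI and score manager, then installs turn-begin, turn-end and unit-death handlers on the teams.
; It passes the first "Player"-tagged actor, cast to SpawnerTeamLeader, to a new BP_UnitDeploymentGUI in the viewport.
; The three team handlers only forward to the parent class.
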(event EventBeginPlay
  (CallFunction|FindAIandConstructScoreManager)
  (CallFunction|FindTeamsandInstallHandlers (delegate EventAttendTurnBegin) (delegate EventAttendEndOfTurn) (delegate EventAttendDeath))
  (bind _outactors (Actor|GetAllActorswithTag "Player"))
  (bind _asspawner_team_leader (Utilities|Casting|CastToSpawnerTeamLeader (Utilities|Array|Get(acopy) _outactors)))
  (bind _returnvalue (UserInterface|CreateWidget "/Game/Blueprints/UserInterface/Gameplay/BP_UnitDeploymentGUI.BP_UnitDeploymentGUI_C"))
  (Default|AddTeam _returnvalue _asspawner_team_leader)
  (UserInterface|Viewport|AddtoViewport _returnvalue 0))

(event EventAttendTurnBegin
  (params (Team :type Team%20Leader%20Object%20Reference))
  (|CallParentFunction Team))

(event EventAttendEndOfTurn
  (params (Team :type Team%20Leader%20Object%20Reference))
  (|CallParentFunction Team))

(event EventAttendDeath
  (params (Unit :type Unit%20Object%20Reference) (Team :type Team%20Leader%20Object%20Reference))
  (|CallParentFunction Unit Team))

(fn ConstructionScript
  (|CallParentFunction))