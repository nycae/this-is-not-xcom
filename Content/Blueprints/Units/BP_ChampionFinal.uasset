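; Champion unit Blueprint that animates movement and attacks on request.
; PlayMovementAnimation stores a movement list that PlayMovement consumes one step at a time, re-calling itself until empty.
; Each step runs timeline-driven location and rotation interpolation in parallel, turning only when Facing is not Forward, and sets Speed while moving.
; PlayAttackAnimation rotates toward the given direction on its own timeline, then plays a non-looping mesh animation.
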(event Custom|Play%20Movement
  (bind _turnmovements (Variables|Default|GetTurnMovements))
  (bind _output (Utilities|Array|Get(acopy) _turnmovements))
  (Utilities|FlowControl|Sequence
    (:then_0
      (if (not (Utilities|Enum|Equal(Enum) (Variables|Default|GetFacing) "DE_Forward"))
        (bind _progression (Timeline|Timeline_1 PlayFromStart)
          (:Update
            (bind _rotator (CallFunction|GetRotator _output))
            (Transformation|SetActorRotation (Math|Interpolation|RInterpTo (Transformation|GetActorRotation) _rotator _progression 1.0)))
          (:Finished
            (Variables|Default|SetFacing (Utilities|Enum|ByteToEnumEDirectionEnum _output))))))
    (:then_1
      (bind _output_get (Variables|Default|SetOrigin (Transformation|GetActorLocation)))
      (Variables|Default|SetSpeed 1e+02)
      (bind _result (CallFunction|GetPosition _output))
      (bind _animcurve (Timeline|Timeline_0 PlayFromStart)
        (:Update
          (Transformation|SetActorLocation (Math|Interpolation|VInterpTo _output_get _result _animcurve 1.0) false false))
        (:Finished
          (Variables|Default|SetSpeed 0.0)
          (Variables|Default|SetOrigin (Math|Interpolation|VInterpTo _output_get _result _animcurve 1.0))
          (Utilities|Array|RemoveIndex _turnmovements)
          (if (> (Utilities|Array|Length _turnmovements) 0)
            (CallFunction|PlayMovement)))))))

(event EventBeginPlay)

(event Collision|EventActorBeginOverlap
  (params (OtherActor :type Actor%20Object%20Reference)))

(event EventTick
  (params (DeltaSeconds :type Float%20%28single-precision%29)))

(event EventPlayAttackAnimation
  (params (Direction :type EDirectionEnum%20Enum :default "DE_Forward"))
  (Timeline|Timeline_2 PlayFromStart
    (:Update
      (bind _rotator (CallFunction|GetRotator Direction))
      (Transformation|SetActorRotation (Math|Interpolation|RInterpTo (Transformation|GetActorRotation) _rotator 0.0 0.0)))
    (:Finished
      (Components|Animation|PlayAnimation (Variables|Character|GetMesh) 0 false))))

(event EventPlayMovementAnimation
  (params (MovementList :type Array%20of%20EDirectionEnum%20Enums :default "DE_Forward"))
  (Variables|Default|SetTurnMovements MovementList)
  (CallFunction|PlayMovement))

(fn ConstructionScript)