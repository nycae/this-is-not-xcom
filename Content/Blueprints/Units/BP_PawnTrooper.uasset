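; Trooper unit pawn that plays back a queued list of four-direction moves, one 100-unit step at a time.
; PlayMovement runs a move timeline alongside a rotation timeline, which plays only when Facing is not Forward.
; Timeline curves drive VInterpTo and RInterpTo toward targets from GetPosition and GetRotator.
; Speed is set during each step, and each finished move pops the queue and recurses until it empties.
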(event Custom|PlayMovement
  (bind _turnmovements (Variables|Default|GetTurnMovements))
  (bind _output (Utilities|Array|Get(acopy) _turnmovements))
  (Utilities|FlowControl|Sequence
    (:then_0
      (if (not (Utilities|Enum|Equal(Enum) (Variables|Default|GetFacing) "DE_Forward"))
        (bind _progression (Timeline|TimlineRotate PlayFromStart)
          (:Update
            (bind _rotator (CallFunction|GetRotator _output))
            (Transformation|SetActorRotation (Math|Interpolation|RInterpTo (Transformation|GetActorRotation) _rotator _progression 1.0)))
          (:Finished
            (Variables|Default|SetFacing (Utilities|Enum|ByteToEnumEDirectionEnum _output))))))
    (:then_1
      (bind _output_get (Variables|Default|SetOrigin (Transformation|GetActorLocation)))
      (Variables|Default|SetSpeed 1e+02)
      (bind _result (CallFunction|GetPosition _output))
      (bind _animcurve (Timeline|TimelineMove PlayFromStart)
        (:Update
          (Transformation|SetActorLocation (Math|Interpolation|VInterpTo _output_get _result _animcurve 1.0) false false))
        (:Finished
          (Variables|Default|SetSpeed 0.0)
          (Variables|Default|SetOrigin (Math|Interpolation|VInterpTo _output_get _result _animcurve 1.0))
          (Utilities|Array|RemoveIndex _turnmovements)
          (if (> (Utilities|Array|Length _turnmovements) 0)
            (CallFunction|PlayMovement)))))))

(event EventBeginPlay)

(event Collision|EventActorBeginOverlap
  (params (OtherActor :type Actor%20Object%20Reference)))

(event EventTick
  (params (DeltaSeconds :type Float%20%28single-precision%29)))

(event EventPlayMovementAnimation
  (params (MovementList :type Array%20of%20EDirectionEnum%20Enums :default "DE_Forward"))
  (Variables|Default|SetTurnMovements MovementList)
  (CallFunction|PlayMovement))

(fn ConstructionScript)

(fn GetRotator
  (params (direction :type Byte))
  (switch Utilities|FlowControl|Switch|Switchon direction
    (:DE_Forward
      (return "0,0.100000, 0"))
    (:DE_Backward
      (return "0.000000,180.000000,0.000000"))
    (:DE_Left
      (return "0.000000,270.000000,0.000000"))
    (:DE_Right
      (return "0.000000,90.000000,0.000000"))))

(fn GetPosition
  (params (Direction :type Byte))
  (bind _origin (Variables|Default|GetOrigin))
  (bind (_x _y _z) (Math|Vector|BreakVector _origin))
  (bind (_x_2 _y_2 _z_2) (Math|Vector|BreakVector _origin))
  (bind (_x_3 _y_3 _z_3) (Math|Vector|BreakVector _origin))
  (bind (_x_4 _y_4 _z_4) (Math|Vector|BreakVector _origin))
  (switch Utilities|FlowControl|Switch|Switchon Direction
    (:DE_Forward
      (return (Math|Vector|MakeVector (+ _x_2 1e+02) _y_2 _z_2)))
    (:DE_Backward
      (return (Math|Vector|MakeVector (- _x_3 1e+02) _y_3 _z_3)))
    (:DE_Left
      (return (Math|Vector|MakeVector _x_4 (- _y_4 1e+02) _z_4)))
    (:DE_Right
      (return (Math|Vector|MakeVector _x (+ _y 1e+02) _z)))))