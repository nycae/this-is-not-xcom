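; Trooper unit pawn for a tile-based game, setting its move range, health and attack stats in the construction script.
; Movement consumes a direction list recursively, with timelines turning the pawn while sliding it one tile, sized by MapGenerator, per step.
; Attacks turn the pawn toward a direction, then play a mesh animation.
; Tick updates the health bar widget and hides it when the trooper is dead.
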(event Custom|Play%20Movement
  (bind _turnmovements (Variables|Default|GetTurnMovements))
  (bind _turnmovements_2 (Variables|Default|GetTurnMovements))
  (bind _output (Utilities|Array|Get(acopy) _turnmovements))
  (Utilities|FlowControl|Sequence
    (:then_0
      (if (Utilities|Enum|NotEqual(Enum) (Variables|Default|GetFacing) (Utilities|Enum|ByteToEnumEDirectionEnum _output))
        (bind _progression (Timeline|Timeline_1 PlayFromStart)
          (:Update
            (Transformation|SetActorRotation (Math|Interpolation|RInterpTo (Transformation|GetActorRotation) (Class|Trooper|GetRotationbyDirection (Utilities|Enum|ByteToEnumEDirectionEnum _output)) _progression 1.0)))
          (:Finished
            (if (> (Utilities|Array|Length _turnmovements_2) 0)
              (Variables|Default|SetFacing (Utilities|Array|Get(acopy) _turnmovements_2)))))))
    (:then_1
      (bind _outactors (Actor|GetAllActorsOfClass "/Script/ThisisNotXcom.MapGenerator"))
      (bind _output_get (Variables|Default|SetOrigin (Transformation|GetActorLocation)))
      (Variables|Default|SetSpeed 1e+02)
      (bind _returnvalue (CallFunction|ExecuteJustOnce (Utilities|Enum|ByteToEnumEDirectionEnum _output) (Variables|/Script/ThisisNotXcom.MapGenerator|GetTileSize (Utilities|Array|Get(acopy) _outactors))))
      (bind _animcurve (Timeline|Timeline_0 PlayFromStart)
        (:Update
          (Transformation|SetActorLocation (Math|Interpolation|VInterpTo _output_get _returnvalue _animcurve 1.0) false false))
        (:Finished
          (Variables|Default|SetSpeed 0.0)
          (Variables|Default|SetOrigin (Math|Interpolation|VInterpTo _output_get _returnvalue _animcurve 1.0))
          (Utilities|Array|RemoveIndex _turnmovements)
          (if (> (Utilities|Array|Length _turnmovements) 0)
            (CallFunction|PlayMovement)))))))

(event EventBeginPlay)

(event Collision|EventActorBeginOverlap
  (params (OtherActor :type Actor%20Object%20Reference)))

(event EventTick
  (params (DeltaSeconds :type Float%20%28single-precision%29))
  (bind _asbp_trooper_health (Utilities|Casting|CastToBP_TrooperHealth (UserInterface|GetUserWidgetObject (Variables|Default|GetWidget))))
  (Progress|SetPercent (Variables|/Game/Blueprints/UserInterface/BP_TrooperHealth.BP_TrooperHealth_C|GetProgressBar_82 _asbp_trooper_health) (Class|Trooper|GetHealthPercentage))
  (if (Variables|Default|GetbIsDead)
    (Rendering|SetVisibility (Variables|Default|GetWidget) false true)))

(event EventPlayAttackAnimation
  (params (Direction :type EDirectionEnum%20Enum :default "DE_Forward"))
  (Timeline|Timeline_2 PlayFromStart
    (:Update
      (Transformation|SetActorRotation (Math|Interpolation|RInterpTo (Transformation|GetActorRotation) (Class|Trooper|GetRotationbyDirection Direction) 0.0 0.0)))
    (:Finished
      (Components|Animation|PlayAnimation (Variables|Character|GetMesh) 0 false))))

(event EventPlayMovementAnimation
  (params (MovementList :type Array%20of%20EDirectionEnum%20Enums :default "DE_Forward"))
  (Variables|Default|SetTurnMovements MovementList)
  (CallFunction|PlayMovement))

(event EventDestroyed)

(fn ConstructionScript
  (Variables|Default|SetMaxMoveDepth 2)
  (bind _output_get (Variables|Default|SetMaxHealth 200))
  (Variables|Default|SetHealth _output_get)
  (Variables|Default|SetAttackDamage 50)
  (Variables|Default|SetMaxAttackDepth 1))

(fn ExecuteJustOnce
  (params (Dir :type EDirectionEnum%20Enum :default "DE_Forward") (Size :type Integer))
  (return (Class|Trooper|GetVectorfromDirection Dir Size)))