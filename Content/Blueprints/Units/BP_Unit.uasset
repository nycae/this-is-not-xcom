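; BP_Unit is a grid-based unit actor that animates tile movement, turning and attacks, and plays an error voice line.
; A queue of directions is consumed one tile per Move timeline, using the Grid's TileSize, while turning runs alongside as needed.
; Attacks rotate the unit on a separate timeline before playing the montage.
; A health bar widget is linked to the unit and shown only on cursor hover.
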(event Custom|Play%20Movement
  (bind _turnmovements (Variables|Default|GetTurnMovements))
  (bind _turnmovements_2 (Variables|Default|GetTurnMovements))
  (bind _output (Utilities|Array|Get(acopy) _turnmovements))
  (if (> (Utilities|Array|Length _turnmovements) 0)
    (if (Utilities|Enum|Equal(Enum) (Variables|Default|GetFacing) _output)
      _
      (else
        (CallFunction|Turnto _output)))
    (bind _outactors (Actor|GetAllActorsOfClass "/Script/ThisisNotXcom.Grid"))
    (bind _output_get (Variables|Default|SetOrigin (Transformation|GetActorLocation)))
    (bind _new_position (CallFunction|CalculateNewPosition _output (Variables|/Script/ThisisNotXcom.Grid|GetTileSize (Utilities|Array|Get(acopy) _outactors))))
    (bind _progression (Timeline|Move PlayFromStart)
      (:Update
        (Transformation|SetActorLocation (Math|Interpolation|VInterpTo _output_get _new_position _progression 1.0) false false))
      (:Finished
        (Utilities|Array|RemoveIndex _turnmovements_2)
        (if (> (Utilities|Array|Length _turnmovements_2) 0)
          (CallFunction|PlayMovement)
          (else
            (Class|Unit|PlayIdleAnimation)))))))

(event Custom|Turn%20To
  (params (New%20direction :type EDirectionEnum%20Enum :default "DE_Forward"))
  (bind _lineal (Timeline|Turning PlayFromStart)
    (:Update
      (Transformation|SetActorRotation (Math|Interpolation|RInterpTo (Transformation|GetActorRotation) (Class|Unit|GetRotationbyDirection New%20direction) _lineal 0.5)))
    (:Finished
      (Variables|Default|SetFacing New%20direction))))

(event EventBeginPlay
  (bind _healthbar (Variables|Default|GetHealthBar))
  (bind _asbp_trooper_stats (Utilities|Casting|CastToBP_TrooperStats (UserInterface|GetUserWidgetObject _healthbar)))
  (Variables|/Game/Blueprints/UserInterface/BP_TrooperStats.BP_TrooperStats_C|SetOwning%20Actor _asbp_trooper_stats self)
  (Rendering|SetVisibility _healthbar false true))

(event Collision|EventActorBeginOverlap
  (params (OtherActor :type Actor%20Object%20Reference)))

(event EventTick
  (params (DeltaSeconds :type Float%20%28single-precision%29)))

(event EventPlayMovementAnimation
  (params (MovementList :type Array%20of%20EDirectionEnum%20Enums :default "DE_Forward"))
  (Variables|Default|SetTurnMovements MovementList)
  (Class|Unit|PlayRunAnimation)
  (CallFunction|PlayMovement))

(event EventPlayAttackAnimation
  (params (Direction :type EDirectionEnum%20Enum :default "DE_Forward"))
  (bind _lineal (Timeline|Turning2 Play)
    (:Update
      (Transformation|SetActorRotation (Math|Interpolation|RInterpTo (Transformation|GetActorRotation) (Class|Unit|GetRotationbyDirection Direction) _lineal 0.5)))
    (:Finished
      (Variables|Default|SetFacing Direction)
      (Class|Unit|PlayAttackMontage))))

(event EventPlayErrorSpeech
  (Audio|Components|Audio|Play (Variables|Default|GetDoesNotCompute) 0.0))

(event MouseInput|EventActorBeginCursorOver
  (Rendering|SetVisibility (Variables|Default|GetHealthBar) true true))

(event MouseInput|EventActorEndCursorOver
  (Rendering|SetVisibility (Variables|Default|GetHealthBar) false true))

(fn ConstructionScript)

(fn CalculateNewPosition
  (params (Direction :type EDirectionEnum%20Enum :default "DE_Forward") (Tile%20Size :type Integer))
  (return (Class|Unit|GetVectorfromDirection Direction Tile%20Size)))